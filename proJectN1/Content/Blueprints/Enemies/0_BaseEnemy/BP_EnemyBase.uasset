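; BP_EnemyBase is a base enemy that takes and deals damage, shows a health bar widget and is destroyed at zero health or when the player is destroyed.
; Each hit updates the widget, reports a damage event for AI, flashes the sprite's dynamic material, briefly freezes the enemy via time dilation and knocks it back along the player's forward vector.
; A DoOnce gate, reset after a hit-stun delay, blocks repeated damage.
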(event `self.ReceiveBeginPlay`
  ;[1 1 1] Event Begin Play
  (bind _asbp_player (cast `/Game/Blueprints/Player/BP_Player` (`GameplayStatics.GetPlayerCharacter` 0)))
  (bind _output_get (set `self.Player Ref` _asbp_player))
  (add `self.OnDestroyed` _output_get (delegate `On Player Dead`))
  ;;[1 1 1] Set Dynamic Material for Flash When Hit
  (bind _returnvalue (`PrimitiveComponent.CreateDynamicMaterialInstance` (`self.Sprite`) 0 null "None"))
  (bind _output_get_2 (set `self.Dynamic Material Ref` _returnvalue))
  (`MaterialInstanceDynamic.SetScalarParameterValue` _output_get_2 "FlashMultiplier" 0.2)
  (bind _aswbp_enemy_health (cast `/Game/Blueprints/Widgets/Enemies/WBP_EnemyHealth` (`WidgetComponent.GetUserWidgetObject` (`self.Health Bar`))))
  (set `self.Enemy Health Ref` _aswbp_enemy_health)
  (set `/Game/Blueprints/Widgets/Enemies/WBP_EnemyHealth.Widget Health` (`self.Current Health`) (`self.Enemy Health Ref`)))

(event `On Player Dead` :!signature `self.OnDestroyed`
  (params (DestroyedActor :type "Actor Object Reference"))
  ;[1 1 1] Event Begin Play
  (`self.K2_DestroyActor`))

(event `self.ReceiveAnyDamage`
  (params (Damage :type "Float (single-precision)") (DamageType :type "DamageType Object Reference") (InstigatedBy :type "Controller Object Reference") (DamageCauser :type "Actor Object Reference"))
  (bind _returnvalue (- (`self.Current Health`) Damage))
  ;[1 1 1] Calculate Damage Recieve and reports damage event for AI
  (`/Engine/EditorBlueprintResources/StandardMacros.DoOnce` false :!label _label
    (:`Completed`
      (bind _output_get (set `self.Current Health` (`KismetMathLibrary.FClamp` _returnvalue 0.0 _returnvalue)))
      (set `/Game/Blueprints/Widgets/Enemies/WBP_EnemyHealth.Widget Health` _output_get (`self.Enemy Health Ref`))
      (`AISense_Damage.ReportDamageEvent` self (`self.Player Ref`) Damage (`self.K2_GetActorLocation` (`self.Player Ref`)))
      (`MaterialInstanceDynamic.SetScalarParameterValue` (`self.Dynamic Material Ref`) "FlashMultiplier" 1.0)
      (`|ExecutionSequence`
        (:`then_0`
          (if (== _output_get 0.0)
            ;[0.3062 1 0.4374] Enemy is Defeated
            (set `self.Is defeated` true)
            (if (`self.Is defeated`)
              (`self.K2_DestroyActor`))
            (else
              (`KismetSystemLibrary.Delay` (`self.Hit Stun Delay`))
              (`self.Reset Damage System`))))
        (:`then_1`
          (`self.Hit Stop`)
          ;[1 1 1] Knockback Enemy when Hit
          (`KismetSystemLibrary.MoveComponentTo` (`self.CapsuleComponent`) (+ (`self.K2_GetActorLocation`) (* (`self.GetActorForwardVector` (`self.Player Ref`)) (`self.KnockbackDistance`))) (`self.K2_GetActorRotation`)))))))

(event `Reset Damage System`
  ;[1 1 1] Calculate Damage Recieve and reports damage event for AI
  (goto _label :!via `Reset`))

(event `Hit Stop`
  ;[1 1 1] Reset Hit Stop
  (set `self.CustomTimeDilation` 0.0)
  (`KismetSystemLibrary.RetriggerableDelay` (`self.Hit Stop Delay`))
  (set `self.CustomTimeDilation` 1.0)
  (`MaterialInstanceDynamic.SetScalarParameterValue` (`self.Dynamic Material Ref`) "FlashMultiplier" 0.2))

(event `/Game/Blueprints/Player/BPI_Interactions.Damage Player`
  ;[1 1 1] Damage Player
  (`GameplayStatics.ApplyDamage` (`self.Player Ref`) (`self.Current Damage`)))

(fn `UserConstructionScript`
  (set `self.Current Health` (`self.Max Health`))
  (set `self.Current Damage` (`self.Max Damage`)))
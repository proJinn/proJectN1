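; Base enemy projectile that damages the player on contact and destroys itself.
; On BeginPlay it caches the BP_Player reference and starts a three-second lifetime before self-destruction.
; Each tick it traces on the Visibility channel from the actor to its TraceEnd component, destroying itself on any hit.
; HitBox overlap applies ProjectileDamage only to the cached player, then destroys the projectile.
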(event `self.ReceiveTick`
  (params (DeltaSeconds :type "Float (single-precision)"))
  (bind (_outhit _returnvalue) (`KismetSystemLibrary.LineTraceSingle` (`self.K2_GetActorLocation`) (`SceneComponent.K2_GetComponentLocation` (`self.Trace End`)) "TraceTypeQuery1"))
  (if _returnvalue
    (`self.K2_DestroyActor` :!label _label)))

(event `self.HitBox.OnComponentBeginOverlap`
  (params (OverlappedComponent :type "PrimitiveComponent Object Reference") (OtherActor :type "Actor Object Reference") (OtherComp :type "PrimitiveComponent Object Reference") (OtherBodyIndex :type Integer) (bFromSweep :type Boolean) (SweepResult :type "HitResult Structure (by ref)"))
  (if (== OtherActor (`self.Player Ref`))
    (`GameplayStatics.ApplyDamage` (`self.Player Ref`) (`self.Projectile Damage`))
    (goto _label)))

(event `self.ReceiveBeginPlay`
  (bind _asbp_player (cast `/Game/Blueprints/Player/BP_Player` (`GameplayStatics.GetPlayerCharacter` 0)))
  (set `self.Player Ref` _asbp_player)
  (`KismetSystemLibrary.Delay` 3.0)
  (goto _label))

(fn `UserConstructionScript`)
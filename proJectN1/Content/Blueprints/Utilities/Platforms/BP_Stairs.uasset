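; BP_Stairs is a climbable ladder volume that lets BP_Player move vertically while inside its Box trigger.
; Overlapping the Box sets the player's InsideLadder flag and switches movement to Flying; leaving clears it and switches to Falling.
; It caches the player on BeginPlay and, when that player is destroyed, reruns the lookup to re-cache and rebind to the current player character.
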(event `Begin Play Reset`
  (bind _asbp_player (cast `/Game/Blueprints/Player/BP_Player` (`GameplayStatics.GetPlayerCharacter` 0) :!label _label))
  (bind _output_get (set `self.Player Ref` _asbp_player))
  (add `self.OnDestroyed` _output_get (delegate `Reset When Player Dies`)))

(event `self.ReceiveBeginPlay`
  (goto _label))

(event `Reset When Player Dies` :!signature `self.OnDestroyed`
  (params (DestroyedActor :type "Actor Object Reference"))
  (`self.Begin Play Reset`))

(event `self.Box.OnComponentBeginOverlap`
  (params (OverlappedComponent :type "PrimitiveComponent Object Reference") (OtherActor :type "Actor Object Reference") (OtherComp :type "PrimitiveComponent Object Reference") (OtherBodyIndex :type Integer) (bFromSweep :type Boolean) (SweepResult :type "HitResult Structure (by ref)"))
  (if (== OtherActor (`self.Player Ref`))
    (set `/Game/Blueprints/Player/BP_Player.Inside Ladder?` true (`self.Player Ref`))
    (`CharacterMovementComponent.SetMovementMode` (`Character.CharacterMovement` (`self.Player Ref`)) "MOVE_Flying" 0)
    (`KismetSystemLibrary.PrintString` "Inside Ladder")))

(event `self.Box.OnComponentEndOverlap`
  (params (OverlappedComponent :type "PrimitiveComponent Object Reference") (OtherActor :type "Actor Object Reference") (OtherComp :type "PrimitiveComponent Object Reference") (OtherBodyIndex :type Integer))
  (if (== OtherActor (`self.Player Ref`))
    (set `/Game/Blueprints/Player/BP_Player.Inside Ladder?` false (`self.Player Ref`))
    (`CharacterMovementComponent.SetMovementMode` (`Character.CharacterMovement` (`self.Player Ref`)) "MOVE_Falling" 0)))

(fn `UserConstructionScript`)
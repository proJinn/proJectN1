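; BP_NewPlatformPosSaver is a checkpoint-style trigger that saves a new platform position on the player.
; When the player overlaps ReferenceCollision, it copies its own transform into the player's NewPlatformTransform, prints it and calls SetPlatformLocation.
; It caches the BP_Player reference on BeginPlay and binds to its OnDestroyed event, re-running the lookup and binding when that player is destroyed.
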(event `self.ReceiveBeginPlay`
  (bind _asbp_player (cast `/Game/Blueprints/Player/BP_Player` (`GameplayStatics.GetPlayerCharacter` 0) :!label _label))
  (bind _output_get (set `self.Player Ref` _asbp_player))
  (add `self.OnDestroyed` _output_get (delegate `Reset When Player Dies`)))

(event `Reset When Player Dies` :!signature `self.OnDestroyed`
  (params (DestroyedActor :type "Actor Object Reference"))
  (goto _label))

(event `self.Reference Collision.OnComponentBeginOverlap`
  (params (OverlappedComponent :type "PrimitiveComponent Object Reference") (OtherActor :type "Actor Object Reference") (OtherComp :type "PrimitiveComponent Object Reference") (OtherBodyIndex :type Integer) (bFromSweep :type Boolean) (SweepResult :type "HitResult Structure (by ref)"))
  (`/Engine/EditorBlueprintResources/StandardMacros.IsValid` (`self.Player Ref`)
    (:`Is Valid`
      (if (== OtherActor (`self.Player Ref`))
        (bind _output_get (set `/Game/Blueprints/Player/BP_Player.New Platform Transform` (`self.GetTransform`) (`self.Player Ref`)))
        (`KismetSystemLibrary.PrintString` (`KismetStringLibrary.Conv_TransformToString` _output_get))
        (`/Game/Blueprints/Player/BP_Player.Set Platform Location` (`self.Player Ref`))))))

(fn `UserConstructionScript`)
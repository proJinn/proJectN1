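; BP_CheckPoint is a one-shot checkpoint that sets the player's respawn position in the action platformer game mode.
; When the player overlaps its collision, it writes its own transform to GM_ActionPlatformer's PlayerRespawnPos, prints a debug message and destroys itself.
; It caches player and game mode references on BeginPlay, and reruns that setup when the player is destroyed to pick up the current pawn.
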(event `Begin Play Reset`
  (bind _asbp_player (cast `/Game/Blueprints/Player/BP_Player` (`GameplayStatics.GetPlayerCharacter` 0) :!label _label))
  (set `self.Player Ref` _asbp_player)
  (bind _asgm_action_platformer (cast `/Game/Blueprints/Player/GM_ActionPlatformer` (`GameplayStatics.GetGameMode`)))
  (set `self.Game Mode Ref` _asgm_action_platformer)
  (add `self.OnDestroyed` (`self.Player Ref`) (delegate `Reset When Player Dies`)))

(event `self.ReceiveBeginPlay`
  (goto _label))

(event `Reset When Player Dies` :!signature `self.OnDestroyed`
  (params (DestroyedActor :type "Actor Object Reference"))
  (`self.Begin Play Reset`))

(event `self.Reference Collision.OnComponentBeginOverlap`
  (params (OverlappedComponent :type "PrimitiveComponent Object Reference") (OtherActor :type "Actor Object Reference") (OtherComp :type "PrimitiveComponent Object Reference") (OtherBodyIndex :type Integer) (bFromSweep :type Boolean) (SweepResult :type "HitResult Structure (by ref)"))
  (if (== OtherActor (`self.Player Ref`))
    (`/Engine/EditorBlueprintResources/StandardMacros.DoOnce` false
      (:`Completed`
        (set `/Game/Blueprints/Player/GM_ActionPlatformer.Player Respawn Pos` (`self.GetTransform`) (`self.Game Mode Ref`))
        (`KismetSystemLibrary.PrintString` (`KismetStringLibrary.Concat_StrStr` "New " "Respawn " "Position"))
        (`self.K2_DestroyActor`)))))

(fn `UserConstructionScript`)
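; BP_EndlessPit is a pit hazard that damages the player who falls into its Box trigger and returns them to a platform.
; On overlap it applies damage, launches the player with both velocity overrides, then after a short delay snaps the capsule to the player's NewPlatformTransform via a zero-time MoveComponentTo.
; It caches the player on BeginPlay and binds to its OnDestroyed to re-run that lookup when the player is destroyed.
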(event `self.ReceiveBeginPlay`
  (bind _asbp_player (cast `/Game/Blueprints/Player/BP_Player` (`GameplayStatics.GetPlayerCharacter` 0) :!label _label))
  (bind _output_get (set `self.Player Ref` _asbp_player))
  (add `self.OnDestroyed` _output_get (delegate `Reset When Player Dies`)))

(event `Reset When Player Dies` :!signature `self.OnDestroyed`
  (params (DestroyedActor :type "Actor Object Reference"))
  (goto _label))

(event `self.Box.OnComponentBeginOverlap`
  (params (OverlappedComponent :type "PrimitiveComponent Object Reference") (OtherActor :type "Actor Object Reference") (OtherComp :type "PrimitiveComponent Object Reference") (OtherBodyIndex :type Integer) (bFromSweep :type Boolean) (SweepResult :type "HitResult Structure (by ref)"))
  (bind (_new_platform_transform_location _new_platform_transform_rotation) (`KismetMathLibrary.BreakTransform` (`/Game/Blueprints/Player/BP_Player.New Platform Transform` (`self.Player Ref`))))
  (`/Engine/EditorBlueprintResources/StandardMacros.IsValid` (`self.Player Ref`)
    (:`Is Valid`
      (if (== OtherActor (`self.Player Ref`))
        (`GameplayStatics.ApplyDamage` (`self.Player Ref`) (`self.Base Damage`))
        (`Character.LaunchCharacter` (`self.Player Ref`) (`self.Launch Velocity`) true true)
        (`KismetSystemLibrary.Delay` 0.3)
        (`KismetSystemLibrary.MoveComponentTo` (`Character.CapsuleComponent` (`self.Player Ref`)) _new_platform_transform_location _new_platform_transform_rotation false false 0.0)))))

(fn `UserConstructionScript`)
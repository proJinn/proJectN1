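; BP_BossDoor is a boss arena door that closes when the player enters its trigger and reopens when the player is destroyed.
; On overlap, it disables input, spawns BossToSpawn, teleports the player and closes via timeline-driven Lerp.
; Once closed, it restores input after a short delay and resets the DoOnce.
; Player destruction re-runs the player binding and opens the door; the construction script positions the boss spawn from BossPos.
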(event `Reset Begin Play`
  (bind _asbp_player (cast `/Game/Blueprints/Player/BP_Player` (`GameplayStatics.GetPlayerCharacter` 0) :!label _label))
  (bind _output_get (set `self.Player Ref` _asbp_player))
  (add `self.OnDestroyed` _output_get (delegate `Reset When Player Dies`)))

(event `self.ReceiveBeginPlay`
  (goto _label))

(event `Reset When Player Dies` :!signature `self.OnDestroyed`
  (params (DestroyedActor :type "Actor Object Reference"))
  (`self.Reset Begin Play`)
  (bind (_direction _alpha) (`Timeline|Open Door When Player Dies` :!via `PlayFromStart`)
    (:`Update`
      (`SceneComponent.K2_SetRelativeLocation` (`self.Door`) (`KismetMathLibrary.VLerp` (`SceneComponent.RelativeLocation` (`self.Door`)) (`self.Opened Door Location`) _alpha) false false))))

(event `self.Trigger Door.OnComponentBeginOverlap`
  (params (OverlappedComponent :type "PrimitiveComponent Object Reference") (OtherActor :type "Actor Object Reference") (OtherComp :type "PrimitiveComponent Object Reference") (OtherBodyIndex :type Integer) (bFromSweep :type Boolean) (SweepResult :type "HitResult Structure (by ref)"))
  (bind _player_ref (`self.Player Ref`))
  (if (== OtherActor (`self.Player Ref`))
    (`/Engine/EditorBlueprintResources/StandardMacros.DoOnce` false :!label _label_2
      (:`Completed`
        (`KismetSystemLibrary.PrintString` "Boss Door")
        (`self.DisableInput` (`self.Player Ref`) null)
        (`|SpawnActorFromClass` (`self.Boss to Spawn`) (`SceneComponent.K2_GetComponentToWorld` (`self.Boss Spawn Pos`)) "Undefined" "OverrideRootScale" null null)
        (`self.K2_TeleportTo` _player_ref (`SceneComponent.K2_GetComponentLocation` (`self.Player Teleport Pos`)) (`self.K2_GetActorRotation` _player_ref))
        (bind (_direction _alpha) (`Timeline|Close Door` :!via `PlayFromStart`)
          (:`Update`
            (`SceneComponent.K2_SetRelativeLocation` (`self.Door`) (`KismetMathLibrary.VLerp` (`SceneComponent.RelativeLocation` (`self.Door`)) (`self.Closed Door Location`) _alpha) false false))
          (:`Finished`
            (`KismetSystemLibrary.Delay` 0.5)
            (`self.EnableInput` (`self.Player Ref`) null)
            (`self.Reset Boss Door`)))))))

(event `Reset Boss Door`
  (goto _label_2 :!via `Reset`))

(fn `UserConstructionScript`
  (`SceneComponent.K2_SetRelativeTransform` (`self.Boss Spawn Pos`) (`self.Boss Pos`) false false))
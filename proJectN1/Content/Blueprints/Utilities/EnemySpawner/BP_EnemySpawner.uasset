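; Trigger-box enemy spawner that spawns five configurable enemies when the player leaves its volume.
; Entering the box arms it if all tracked enemy references are invalid; exiting spawns and disarms, though the fifth enemy's reference is never stored.
; Player destruction re-runs setup to fetch and rebind the current player character.
; The Construction Script applies box extent and spawn-point transforms from variables.
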(event `Begin Play Reset`
  (bind _asbp_player (cast `/Game/Blueprints/Player/BP_Player` (`GameplayStatics.GetPlayerCharacter` 0) :!label _label))
  (bind _output_get (set `self.Player Ref` _asbp_player))
  (add `self.OnDestroyed` _output_get (delegate `Reset When Player Dies`)))

(event `self.ReceiveBeginPlay`
  (goto _label))

(event `Reset When Player Dies` :!signature `self.OnDestroyed`
  (params (DestroyedActor :type "Actor Object Reference"))
  (`self.Begin Play Reset`))

(event `self.Trigger Box.OnComponentEndOverlap`
  (params (OverlappedComponent :type "PrimitiveComponent Object Reference") (OtherActor :type "Actor Object Reference") (OtherComp :type "PrimitiveComponent Object Reference") (OtherBodyIndex :type Integer))
  (if (and (== OtherActor (`self.Player Ref`)) (`self.Can Spawn`))
    (set `self.Can Spawn` false)
    (bind _returnvalue (`|SpawnActorFromClass` (`self.Enemy_0`) (`SceneComponent.K2_GetComponentToWorld` (`self.Spawn Ref 1`)) "Undefined" "OverrideRootScale" null null))
    (set `self.Enemy Ref_0` _returnvalue)
    (bind _returnvalue_2 (`|SpawnActorFromClass` (`self.Enemy_1`) (`SceneComponent.K2_GetComponentToWorld` (`self.Spawn Ref 2`)) "Undefined" "OverrideRootScale" null null))
    (set `self.Enemy Ref_1` _returnvalue_2)
    (bind _returnvalue_3 (`|SpawnActorFromClass` (`self.Enemy_2`) (`SceneComponent.K2_GetComponentToWorld` (`self.Spawn Ref 3`)) "Undefined" "OverrideRootScale" null null))
    (set `self.Enemy Ref_2` _returnvalue_3)
    (bind _returnvalue_4 (`|SpawnActorFromClass` (`self.Enemy_3`) (`SceneComponent.K2_GetComponentToWorld` (`self.Spawn Ref 4`)) "Undefined" "OverrideRootScale" null null))
    (set `self.Enemy Ref_3` _returnvalue_4)
    (`|SpawnActorFromClass` (`self.Enemy_4`) (`SceneComponent.K2_GetComponentToWorld` (`self.Spawn Ref 5`)) "Undefined" "OverrideRootScale" null null)))

(event `self.Trigger Box.OnComponentBeginOverlap`
  (params (OverlappedComponent :type "PrimitiveComponent Object Reference") (OtherActor :type "Actor Object Reference") (OtherComp :type "PrimitiveComponent Object Reference") (OtherBodyIndex :type Integer) (bFromSweep :type Boolean) (SweepResult :type "HitResult Structure (by ref)"))
  (if (== OtherActor (`self.Player Ref`))
    (`/Engine/EditorBlueprintResources/StandardMacros.IsValid` (`self.Enemy Ref_0`)
      (:`Is Not Valid`
        (`/Engine/EditorBlueprintResources/StandardMacros.IsValid` (`self.Enemy Ref_1`)
          (:`Is Not Valid`
            (`/Engine/EditorBlueprintResources/StandardMacros.IsValid` (`self.Enemy Ref_2`)
              (:`Is Not Valid`
                (`/Engine/EditorBlueprintResources/StandardMacros.IsValid` (`self.Enemy Ref_3`)
                  (:`Is Not Valid`
                    (`/Engine/EditorBlueprintResources/StandardMacros.IsValid` (`self.Enemy Ref_4`)
                      (:`Is Not Valid`
                        (set `self.Can Spawn` true)))))))))))))

(fn `UserConstructionScript`
  (`BoxComponent.SetBoxExtent` (`self.Trigger Box`) (`self.Spawner Size`) true)
  (`SceneComponent.K2_SetRelativeTransform` (`self.Spawn Ref 1`) (`self.Spawn Pos 1`) false false)
  (`SceneComponent.K2_SetRelativeTransform` (`self.Spawn Ref 2`) (`self.Spawn Pos 2`) false false)
  (`SceneComponent.K2_SetRelativeTransform` (`self.Spawn Ref 3`) (`self.Spawn Pos 3`) false false)
  (`SceneComponent.K2_SetRelativeTransform` (`self.Spawn Ref 4`) (`self.Spawn Pos 4`) false false)
  (`SceneComponent.K2_SetRelativeTransform` (`self.Spawn Ref 5`) (`self.Spawn Pos 5`) false false))
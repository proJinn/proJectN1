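; Trigger volume that blends the view to an assigned fixed camera while the player is inside it, and back to the player on exit.
; Box overlap events drive the view target blend, with box size applied in the construction script.
; On BeginPlay and whenever the player is destroyed, it re-caches the player, rebinds the destroy event and briefly toggles box collision to refresh overlaps.
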(event `Begin Play Reset`
  (`|ExecutionSequence` :!label _label
    (:`then_0`
      (bind _asbp_player (cast `/Game/Blueprints/Player/BP_Player` (`GameplayStatics.GetPlayerCharacter` 0)))
      (bind _output_get (set `self.Player Ref` _asbp_player))
      (add `self.OnDestroyed` _output_get (delegate `Reset When Player Dies`)))
    (:`then_1`
      (`PrimitiveComponent.SetCollisionEnabled` (`self.BoundingBox`) "NoCollision")
      (`KismetSystemLibrary.Delay` 0.0)
      (`PrimitiveComponent.SetCollisionEnabled` (`self.BoundingBox`) "QueryOnly"))))

(event `self.ReceiveBeginPlay`
  (goto _label))

(event `Reset When Player Dies` :!signature `self.OnDestroyed`
  (params (DestroyedActor :type "Actor Object Reference"))
  (`self.Begin Play Reset`))

(event `self.BoundingBox.OnComponentBeginOverlap`
  (params (OverlappedComponent :type "PrimitiveComponent Object Reference") (OtherActor :type "Actor Object Reference") (OtherComp :type "PrimitiveComponent Object Reference") (OtherBodyIndex :type Integer) (bFromSweep :type Boolean) (SweepResult :type "HitResult Structure (by ref)"))
  (if (== OtherActor (`self.Player Ref`))
    (`PlayerController.SetViewTargetWithBlend` (`GameplayStatics.GetPlayerController` 0) (`self.Camera Ref`) (`self.Blend Time`) "VTBlend_Linear" 0.0 false)))

(event `self.BoundingBox.OnComponentEndOverlap`
  (params (OverlappedComponent :type "PrimitiveComponent Object Reference") (OtherActor :type "Actor Object Reference") (OtherComp :type "PrimitiveComponent Object Reference") (OtherBodyIndex :type Integer))
  (if (== OtherActor (`self.Player Ref`))
    (`PlayerController.SetViewTargetWithBlend` (`GameplayStatics.GetPlayerController` 0) (`self.Player Ref`) (`self.Blend Time`) "VTBlend_Linear" 0.0 false)))

(fn `UserConstructionScript`
  (`BoxComponent.SetBoxExtent` (`self.BoundingBox`) (`self.Bounding Box Size`) true))
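; Healing power-up actor that restores a small fixed amount of health to the player.
; Any overlap with its Collision component raises CurrentHealth on PlayerRef, clamped between zero and MaxHealth, then updates the health bar and prints the new value.
; The graph neither checks the overlapping actor, assigns PlayerRef, nor removes the pickup after use.
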(event `self.Collision.OnComponentBeginOverlap`
  (params (OverlappedComponent :type "PrimitiveComponent Object Reference") (OtherActor :type "Actor Object Reference") (OtherComp :type "PrimitiveComponent Object Reference") (OtherBodyIndex :type Integer) (bFromSweep :type Boolean) (SweepResult :type "HitResult Structure (by ref)"))
  (bind _player_ref (`self.Player Ref`))
  (bind _player_ref_2 (`self.Player Ref`))
  (bind _output_get (set `/Game/Blueprints/Player/BP_Player.Current Health` (`KismetMathLibrary.FClamp` (+ (`/Game/Blueprints/Player/BP_Player.Current Health` _player_ref_2) 5.0) 0.0 (`/Game/Blueprints/Player/BP_Player.Max Health` _player_ref_2)) _player_ref))
  (`/Game/Blueprints/Player/BP_Player.Update Health Bar` _player_ref)
  (`KismetSystemLibrary.PrintString` (`KismetStringLibrary.Concat_StrStr` "New " "Health: " (`KismetStringLibrary.Conv_DoubleToString` _output_get))))

(fn `UserConstructionScript`
  (`parent.UserConstructionScript`))
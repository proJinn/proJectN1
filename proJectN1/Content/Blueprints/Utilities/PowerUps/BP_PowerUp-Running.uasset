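; Running power-up that temporarily changes the player's maximum walk speed when its collision component is overlapped.
; The overlap sets PlayerRef's movement to PowerRunSpeed and starts a one-shot timer of PowerUpTime, apparently bound to ResetRunSpeed, which restores the player's StandardRunSpeed.
; The overlap does not check which actor triggered it, and both speed changes print the new value for debugging.
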(event `self.Collision.OnComponentBeginOverlap`
  (params (OverlappedComponent :type "PrimitiveComponent Object Reference") (OtherActor :type "Actor Object Reference") (OtherComp :type "PrimitiveComponent Object Reference") (OtherBodyIndex :type Integer) (bFromSweep :type Boolean) (SweepResult :type "HitResult Structure (by ref)"))
  (bind _output_get (set `CharacterMovementComponent.MaxWalkSpeed` (`self.Power Run Speed`) (`Character.CharacterMovement` (`self.Player Ref`))))
  (`KismetSystemLibrary.K2_SetTimerDelegate` (`|CreateDelegate` :!event `Reset Run Speed`) (`self.Power Up Time`))
  (`KismetSystemLibrary.PrintString` (`KismetStringLibrary.Concat_StrStr` "New " "Run " "Speed: " (`KismetStringLibrary.Conv_DoubleToString` _output_get))))

(fn `Reset Run Speed`
  (bind _player_ref (`self.Player Ref`))
  (bind _output_get (set `CharacterMovementComponent.MaxWalkSpeed` (`/Game/Blueprints/Player/BP_Player.Standard Run Speed` _player_ref) (`Character.CharacterMovement` _player_ref)))
  (`KismetSystemLibrary.PrintString` (`KismetStringLibrary.Concat_StrStr` "Standard " "Run " "Speed: " (`KismetStringLibrary.Conv_DoubleToString` _output_get))))

(fn `UserConstructionScript`
  (`parent.UserConstructionScript`))
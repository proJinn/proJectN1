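; BP_PlayerProjectile is a player projectile that deals damage on overlap and then destroys itself.
; HitBox overlaps apply base damage to the other actor, with the first player controller as instigator.
; Each Tick, a Visibility line trace from the actor to its TraceEnd component destroys it on any hit, without applying damage.
; A three-second delay from BeginPlay limits its lifetime.
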(event `self.ReceiveTick`
  (params (DeltaSeconds :type "Float (single-precision)"))
  (bind (_outhit _returnvalue) (`KismetSystemLibrary.LineTraceSingle` (`self.K2_GetActorLocation`) (`SceneComponent.K2_GetComponentLocation` (`self.Trace End`)) "TraceTypeQuery1"))
  (if _returnvalue
    (`self.K2_DestroyActor` :!label _label)))

(event `self.HitBox.OnComponentBeginOverlap`
  (params (OverlappedComponent :type "PrimitiveComponent Object Reference") (OtherActor :type "Actor Object Reference") (OtherComp :type "PrimitiveComponent Object Reference") (OtherBodyIndex :type Integer) (bFromSweep :type Boolean) (SweepResult :type "HitResult Structure (by ref)"))
  (`GameplayStatics.ApplyDamage` OtherActor (`self.Base Damage`) (`GameplayStatics.GetPlayerController` 0))
  (goto _label))

(event `self.ReceiveBeginPlay`
  (`KismetSystemLibrary.Delay` 3.0)
  (goto _label))

(fn `UserConstructionScript`)
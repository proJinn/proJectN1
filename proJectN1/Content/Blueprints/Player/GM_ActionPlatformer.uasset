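; Game mode for an action platformer that handles player respawning.
; On BeginPlay it caches the player character as BP_Player and sets game-only input.
; RespawnPlayerGM spawns a new actor of the given player's class at the stored PlayerRespawnPos transform and has the first player controller possess it.
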(event `self.ReceiveBeginPlay`
  (bind _asbp_player (cast `/Game/Blueprints/Player/BP_Player` (`GameplayStatics.GetPlayerCharacter` 0)))
  (set `self.Player Ref` _asbp_player)
  (`WidgetBlueprintLibrary.SetInputMode_GameOnly` (`GameplayStatics.GetPlayerController` 0)))

(event `Respawn Player GM`
  (params (Player :type "Character Object Reference"))
  (bind _returnvalue (`|SpawnActorFromClass` (`GameplayStatics.GetObjectClass` Player) (`self.Player Respawn Pos`) "Undefined" "OverrideRootScale" null null))
  (`Controller.Possess` (`GameplayStatics.GetPlayerController` 0) _returnvalue))

(fn `UserConstructionScript`)